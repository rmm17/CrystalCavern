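; BP_Cannon is a cannon actor that fires automatically on a repeating cycle from BeginPlay.
; Each cycle waits for the FireRate delay, then spawns an actor at ProjectileSpawnPoint's location and rotation, scaled by ProjectileScale.
; A timeline then animates the barrel's relative Y position, and its Cannon Fired event track loops execution back to the delay for the next shot.
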(event `self.ReceiveBeginPlay`
  (`KismetSystemLibrary.Delay` (`self.FireRate`) :!label _label)
  (`self.SpawnProjectile`)
  (bind (_direction _barrel_y_offset) (`Timeline|Cannon Barrel Fire Timeline` :`NewTime` 0.0 :!via `PlayFromStart`)
    (:`Update`
      (`SceneComponent.K2_SetRelativeLocation` (`self.CannonBarrel`) (`KismetMathLibrary.MakeVector` 0.0 _barrel_y_offset) false false))
    (:`Cannon Fired`
      (goto _label))))

(fn `SpawnProjectile`
  (bind _projectile_spawn_point (`self.Projectile Spawn Point`))
  (`|SpawnActorFromClass` "/Game/Blueprints/Actors/BP_Projectile.BP_Projectile_C" (`KismetMathLibrary.MakeTransform` (`SceneComponent.K2_GetComponentLocation` _projectile_spawn_point) (`SceneComponent.K2_GetComponentRotation` _projectile_spawn_point) (`KismetMathLibrary.Conv_DoubleToVector` (`self.ProjectileScale`))) "Undefined" "OverrideRootScale" null null))

(fn `UserConstructionScript`)